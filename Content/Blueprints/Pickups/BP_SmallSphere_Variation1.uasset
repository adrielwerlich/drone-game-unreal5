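; Small sphere pickup variation that scales in on spawn and scales out after a lifetime timer.
; Two timelines drive the mesh scale for the wink in and out.
; Collision overlap spawns an explosion emitter at the actor's location, while hits print the other actor's name.
; A random rotation rate is computed at start, but the MoveForward and Rotate helpers are disconnected and Tick is empty, so neither runs.
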(event `self.ReceiveBeginPlay`
  (`self.WinkIn`)
  (set `self.Delta Rotation` (* (`KismetMathLibrary.RandomRotator` false) (`self.RotationScaleFactor`))))

(event `WinkOut`
  (bind (_direction _scale) (`Timeline|WinkOutTimeline`)
    (:`Update`
      (`SceneComponent.SetWorldScale3D` (`self.SphereMesh`) (`KismetMathLibrary.MakeVector` _scale _scale _scale)))))

(event `self.ReceiveTick`
  (params (DeltaSeconds :type "Float (single-precision)")))

(event `WinkIn`
  (bind (_direction _scale) (`Timeline|WinkInTimeline`)
    (:`Update`
      (`SceneComponent.SetWorldScale3D` (`self.SphereMesh`) _scale))))

(event `InitSphereCollisionOnComponentBeginOverlap`
  (add `PrimitiveComponent.OnComponentBeginOverlap` (`self.SphereCollision`) (delegate `OnComponentBeginOverlap_Event`)))

(event `OnComponentBeginOverlap_Event`
  (params (OverlappedComponent :type "PrimitiveComponent Object Reference") (OtherActor :type "Actor Object Reference") (OtherComp :type "PrimitiveComponent Object Reference") (OtherBodyIndex :type Integer) (bFromSweep :type Boolean) (SweepResult :type "HitResult Structure (by ref)"))
  (`GameplayStatics.SpawnEmitterAtLocation` "/Game/FXVarietyPack/Particles/P_ky_explosion.P_ky_explosion" (`self.K2_GetActorLocation`)))

(event `self.SphereCollision.OnComponentHit`
  (params (HitComponent :type "PrimitiveComponent Object Reference") (OtherActor :type "Actor Object Reference") (OtherComp :type "PrimitiveComponent Object Reference") (NormalImpulse :type "Vector Structure") (Hit :type "HitResult Structure (by ref)"))
  (`KismetSystemLibrary.PrintString` (`KismetSystemLibrary.GetDisplayName` OtherActor)))

(fn `UserConstructionScript`)