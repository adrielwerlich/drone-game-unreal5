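; Small sphere pickup that drifts forward while spinning at a random rate and reacts when a BP_CharacterBot overlaps it.
; A looping timer traces downward to hold it at hover height above actors tagged "floor".
; Overlap briefly spawns a heal aura, plays a powerup sound, then scales the sphere out and destroys it.
; A lifetime timer only sets IsWinking, as the wink-out loop timeline is never triggered.
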(event `InitCheckDistanceFromFloor`
  ;[0 0.243 1] CheckDistanceFromFloor-SetInterval/TriggerEventWithTimer.
  (`KismetSystemLibrary.K2_SetTimerDelegate` (delegate `CheckDistanceFromFloor`) 1.0 true))

(event `CheckDistanceFromFloor`
  (bind _returnvalue (`self.K2_GetActorLocation`))
  (bind (_returnvalue_x _returnvalue_y) (`KismetMathLibrary.BreakVector` (`self.K2_GetActorLocation`)))
  (bind (_returnvalue_x_2 _returnvalue_y_2 _returnvalue_z) (`KismetMathLibrary.BreakVector` (+ (`self.DesiredHoverHeight`) (`self.HitLocation`))))
  ;[0 0.243 1] CheckDistanceFromFloor-SetInterval/TriggerEventWithTimer.
  (bind (_outhit _returnvalue_2) (`KismetSystemLibrary.LineTraceSingle` _returnvalue (- _returnvalue (0.0 0.0 1000.0)) "TraceTypeQuery1"))
  (if _returnvalue_2
    (`|ExecutionSequence`
      (:`then_0`
        (bind (_bblockinghit _binitialoverlap _time _distance _location _impactpoint _normal _impactnormal _physmat _hitactor) (`GameplayStatics.BreakHitResult` _outhit))
        (set `self.HitLocation` _impactpoint))
      (:`then_1`
        (bind _output_get (set `self.Hit Actor` _hitactor))
        (for _array_element (`Actor.Tags` _output_get)
          (if (`KismetStringLibrary.Contains` (`KismetStringLibrary.Conv_NameToString` _array_element) "floor")
            (`self.K2_SetActorLocation` (`KismetMathLibrary.MakeVector` _returnvalue_x _returnvalue_y _returnvalue_z))))))))

(event `self.ReceiveTick`
  (params (DeltaSeconds :type "Float (single-precision)"))
  ;[1 1 1] Event Tick
  (if (not (`self.DestroyActor`))
    (`self.K2_AddActorWorldOffset` (* (`self.GetActorForwardVector`) (* DeltaSeconds (`self.Speed`))))
    (`self.K2_AddActorLocalRotation` (* (`self.Delta Rotation`) DeltaSeconds))))

(event `self.ReceiveBeginPlay`
  ;[1 1 1] Begin Play
  (`|ExecutionSequence`
    (:`then_0`
      (`self.InitCheckDistanceFromFloor`))
    (:`then_1`
      (`self.InitSphereCollisionOnComponentBeginOverlap`))
    (:`then_2`
      (`self.WinkIn`))))

(event `WinkIn`
  ;[1 1 1] Begin Play
  (if (`self.DestroyActor`)
    (bind (_direction _scale) (`Timeline|WinkInTimeline` :!via `Stop` :!label _label)
      (:`Update`
        (`SceneComponent.SetWorldScale3D` (`self.SphereMesh`) _scale)
        (set `self.Delta Rotation` (* (`KismetMathLibrary.RandomRotator` false) (`self.RotationScaleFactor`)))
        (`KismetSystemLibrary.K2_SetTimerDelegate` (delegate `InitWinkOutTimelineLoop`) (`self.Lifetime`) false 2.0)))
    (else
      (goto _label))))

(event `InitWinkOutTimelineLoop`
  ;[1 1 1] Begin Play
  (if (not (`self.IsWinking`))
    (set `self.IsWinking` true)))

(event `InitSphereCollisionOnComponentBeginOverlap`
  ;[1 1 1] OnActorOverlapHandler
  (add `PrimitiveComponent.OnComponentBeginOverlap` (`self.SphereCollision`) (delegate `OnComponentBeginOverlap_Event`)))

(event `OnComponentBeginOverlap_Event`
  (params (OverlappedComponent :type "PrimitiveComponent Object Reference") (OtherActor :type "Actor Object Reference") (OtherComp :type "PrimitiveComponent Object Reference") (OtherBodyIndex :type Integer) (bFromSweep :type Boolean) (SweepResult :type "HitResult Structure (by ref)"))
  ;[1 1 1] OnActorOverlapHandler
  (if (`GameplayStatics.ObjectIsA` OtherActor "/Game/Blueprints/Drone/BP_CharacterBot.BP_CharacterBot_C")
    (if (not (`self.DestroyActor`))
      (set `self.DestroyActor` true)
      (bind _returnvalue (`|SpawnActorFromClass` "/Game/FXVarietyPack/Blueprints/BP_ky_healAura.BP_ky_healAura_C" (`self.GetTransform`) "Undefined" "MultiplyWithRoot" null null))
      (`|ExecutionSequence`
        (:`then_0`
          (`GameplayStatics.SpawnSoundAtLocation` "/Game/ImportedStuff/Interface_And_Item_Sounds/Cues/Special_Powerup_05_Cue.Special_Powerup_05_Cue" (`self.K2_GetActorLocation`) (struct) 1.0 1.0 0.0 null null)
          (`KismetSystemLibrary.Delay` 0.1)
          (bind (_direction _scale) (`Timeline|WinkOutTimeline`)
            (:`Update`
              (`SceneComponent.SetWorldScale3D` (`self.SphereMesh`) (`KismetMathLibrary.MakeVector` _scale _scale _scale))
              (`KismetSystemLibrary.Delay` 0.5)
              (`self.K2_DestroyActor`))))
        (:`then_1`
          (`KismetSystemLibrary.Delay` 0.3)
          (`self.K2_DestroyActor` _returnvalue))))))

(fn `UserConstructionScript`)