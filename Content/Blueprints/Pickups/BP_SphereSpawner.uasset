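; Sphere spawner actor that repeatedly spawns an actor of a configurable class at random points within a radius around itself.
; A looping timer started on BeginPlay triggers each spawn after an initial delay.
; Points come from a random direction scaled by a random distance, so spawns cluster toward the center.
; An optional debug sphere, drawn in the construction script and every Tick, shows the spawn radius.
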(event `SpawnSphere`
  ;[1 1 1] Start Random Spawner
  (`|SpawnActorFromClass` (`self.TypeToSpawn`) (`KismetMathLibrary.MakeTransform` (`self.GetRandomPointInSphereRadius`)) "Undefined" "MultiplyWithRoot" null null))

(event `self.ReceiveBeginPlay`
  ;[1 1 1] Start Random Spawner
  (`KismetSystemLibrary.K2_SetTimerDelegate` (delegate `SpawnSphere`) 2.0 true 2.0))

(event `self.ReceiveTick`
  (params (DeltaSeconds :type "Float (single-precision)"))
  (`self.DisplayDebugSphere`))

(fn `DisplayDebugSphere`
  (if (`self.DrawDebugSphere`)
    (`KismetSystemLibrary.DrawDebugSphere` (`self.K2_GetActorLocation`) (`self.SpawnRadius`) 12 (struct :`G` 0.160656 :`B` 1.0 :`A` 1.0) 1.0)))

(fn `GetRandomPointInSphereRadius`
  (returns (RandomPoint :type "Vector Structure"))
  (return (+ (`self.K2_GetActorLocation`) (* (`KismetMathLibrary.GetForwardVector` (`KismetMathLibrary.RandomRotator` false)) (`KismetMathLibrary.RandomFloatInRange` 0.0 (`self.SpawnRadius`))))))

(fn `UserConstructionScript`
  (`self.DisplayDebugSphere`))