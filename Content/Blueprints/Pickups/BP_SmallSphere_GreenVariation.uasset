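; Green variation of a small sphere pickup, built on a parent class, with a glow driven over time.
; Tick accumulates time, and a looping timer sets GlowIntensity by lerping between dim and bright using SanitizeSinXOutput.
; That helper holds nodes remapping the sine of time to 0–1, though they appear unconnected.
; Each timer call creates a new dynamic instance of M_Glow_Green on the mesh rather than reusing one.
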(event `ChangeMaterialGlow`
  (set `self.GlowIntensity` (`KismetMathLibrary.Lerp` 2.0 30.0 (/ (+ (`KismetMathLibrary.Sin` (`self.TimeAccumulator`)) 1.0) 2.0)))
  (bind _returnvalue (`PrimitiveComponent.CreateDynamicMaterialInstance` (`self.SphereMesh`) 0 "/Game/Blueprints/Materials/1/M_Glow_Green.M_Glow_Green" "None"))
  (`MaterialInstanceDynamic.SetScalarParameterValue` _returnvalue "GlowIntensity" (`self.GlowIntensity`)))

(event `self.ReceiveBeginPlay`
  (`parent.ReceiveBeginPlay`)
  (`KismetSystemLibrary.K2_SetTimerDelegate` (delegate `ChangeMaterialGlow`) 0.2 true))

(event `self.ReceiveTick`
  (params (DeltaSeconds :type "Float (single-precision)"))
  (`parent.ReceiveTick` DeltaSeconds)
  (set `self.TimeAccumulator` (+ DeltaSeconds (`self.TimeAccumulator`))))

(fn `UserConstructionScript`
  (`parent.UserConstructionScript`))