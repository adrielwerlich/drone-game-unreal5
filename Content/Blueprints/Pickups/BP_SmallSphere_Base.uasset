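; Base sphere pickup that drifts forward with a random spin and awards a random score when a BP_CharacterBot touches it.
; A looping timer traces downward and resets its hover height over actors tagged as floor.
; Timelines animate mesh scale for wink effects at spawn and on a lifetime timer.
; Pickup spawns particles and sound, increments score through BP_BotPlayerGameMode, then winks out and destroys itself.
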(event `InitCheckDistanceFromFloor`
  ;[0 0.243 1] CheckDistanceFromFloor-SetInterval/TriggerEventWithTimer.
  (`KismetSystemLibrary.K2_SetTimerDelegate` (delegate `CheckDistanceFromFloor`) 10.0 true))

(event `CheckDistanceFromFloor`
  (bind _returnvalue (`self.K2_GetActorLocation`))
  (bind (_returnvalue_x _returnvalue_y) (`KismetMathLibrary.BreakVector` (`self.K2_GetActorLocation`)))
  (bind (_returnvalue_x_2 _returnvalue_y_2 _returnvalue_z) (`KismetMathLibrary.BreakVector` (+ (`self.DesiredHoverHeight`) (`self.HitLocation`))))
  ;[0 0.243 1] CheckDistanceFromFloor-SetInterval/TriggerEventWithTimer.
  (bind (_outhit _returnvalue_2) (`KismetSystemLibrary.LineTraceSingle` _returnvalue (- _returnvalue (0.0 0.0 1000.0)) "TraceTypeQuery1"))
  (if _returnvalue_2
    (`|ExecutionSequence`
      (:`then_0`
        (bind (_bblockinghit _binitialoverlap _time _distance _location _impactpoint _normal _impactnormal _physmat _hitactor) (`GameplayStatics.BreakHitResult` _outhit))
        (set `self.HitLocation` _impactpoint))
      (:`then_1`
        (bind _output_get (set `self.Hit Actor` _hitactor))
        (for _array_element (`Actor.Tags` _output_get)
          (if (`KismetStringLibrary.Contains` (`KismetStringLibrary.Conv_NameToString` _array_element) "floor")
            (`self.K2_SetActorLocation` (`KismetMathLibrary.MakeVector` _returnvalue_x _returnvalue_y _returnvalue_z))))))))

(event `self.ReceiveBeginPlay`
  ;[1 1 1] Begin Play
  (`|ExecutionSequence`
    (:`then_0`
      (`self.InitCheckDistanceFromFloor`))
    (:`then_1`
      (`self.OnSphereBeginOverlap`))
    (:`then_2`
      (`self.WinkIn`))
    (:`then_3`
      (set `self.Score to Add` (`KismetMathLibrary.RandomIntegerInRange` 4 7)))))

(event `self.ReceiveTick`
  (params (DeltaSeconds :type "Float (single-precision)"))
  ;[1 1 1] Event Tick
  (if (not (`self.DestroyActor`))
    (`self.K2_AddActorWorldOffset` (* (`self.GetActorForwardVector`) (* DeltaSeconds (`self.Speed`))))
    (`self.K2_AddActorLocalRotation` (* (`self.DeltaRotation`) DeltaSeconds))))

(event `WinkIn`
  ;[1 1 1] Begin Play
  (if (`self.DestroyActor`)
    (bind (_direction _scale) (`Timeline|Timeline_2` :!via `Stop` :!label _label)
      (:`Update`
        (`SceneComponent.SetWorldScale3D` (`self.SphereMesh`) _scale)
        (set `self.DeltaRotation` (* (`KismetMathLibrary.RandomRotator` false) (`self.RotationScaleFactor`)))
        (`KismetSystemLibrary.K2_SetTimerDelegate` (delegate `InitWinkOutTimelineLoop`) (`self.Lifetime`) false 2.0)))
    (else
      (goto _label))))

(event `InitWinkOutTimelineLoop`
  ;[1 1 1] Begin Play
  (if (not (`self.IsWinking`))
    (set `self.IsWinking` true)
    (bind (_direction _scale) (`Timeline|Timeline`)
      (:`Update`
        (`SceneComponent.SetWorldScale3D` (`self.SphereMesh`) (`KismetMathLibrary.MakeVector` _scale _scale _scale))))))

(event `OnSphereBeginOverlap`
  ;[1 1 1] OnActorOverlapHandler
  (add `PrimitiveComponent.OnComponentBeginOverlap` (`self.SphereCollision`) (delegate `OnComponentBeginOverlap_Event`)))

(event `OnComponentBeginOverlap_Event`
  (params (OverlappedComponent :type "PrimitiveComponent Object Reference") (OtherActor :type "Actor Object Reference") (OtherComp :type "PrimitiveComponent Object Reference") (OtherBodyIndex :type Integer) (bFromSweep :type Boolean) (SweepResult :type "HitResult Structure (by ref)"))
  ;[1 1 1] OnActorOverlapHandler
  (if (`GameplayStatics.ObjectIsA` OtherActor "/Game/Blueprints/Drone/FreeHand/BP_CharacterBot.BP_CharacterBot_C")
    (if (not (`self.DestroyActor`))
      (set `self.DestroyActor` true)
      (bind _returnvalue (`|SpawnActorFromClass` (`self.ParticleSystem_Pickup_ToSpawn_AtOverlap`) (`self.GetTransform`) "Undefined" "MultiplyWithRoot" null null))
      (`|ExecutionSequence`
        (:`then_0`
          (`GameplayStatics.SpawnSoundAtLocation` "/Game/ImportedStuff/Interface_And_Item_Sounds/Cues/Special_Powerup_05_Cue.Special_Powerup_05_Cue" (`self.K2_GetActorLocation`) (struct) 0.2 0.4 0.0 null null)
          (`|ExecutionSequence`
            (:`then_0`
              (`KismetSystemLibrary.Delay` 0.2)
              (bind (_direction _scale__wink_out_timeline) (`Timeline|Timeline_1`)
                (:`Update`
                  (`SceneComponent.SetWorldScale3D` (`self.SphereMesh`) (`KismetMathLibrary.MakeVector` _scale__wink_out_timeline _scale__wink_out_timeline _scale__wink_out_timeline))
                  (`KismetSystemLibrary.Delay` 0.5)
                  (`self.K2_DestroyActor`))))
            (:`then_1`
              (bind _asbp_bot_player_game_mode (cast `/Game/Blueprints/Game/BP_BotPlayerGameMode` (`GameplayStatics.GetGameMode`)))
              (`/Game/Blueprints/Game/BP_BotPlayerGameMode.IncrementScore` _asbp_bot_player_game_mode (`self.Score to Add`)))))
        (:`then_1`
          (`KismetSystemLibrary.Delay` (`self.DelayToDestroy`))
          (`self.K2_DestroyActor` _returnvalue))))))

(fn `UserConstructionScript`
  (set `self.RotationScaleFactor` 0.5))