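; Small sphere challenge pickup Blueprint that explodes and destroys itself when hit by a BP_BlasterBeam actor.
; The actor-hit handler is only bound once the OnSphereBeginOverlap event runs.
; A DestroyActor flag limits the response to one hit, which spawns a particle effect actor, rescales it through a helper function and plays an electric impact sound.
; The pickup then destroys itself after a configurable delay.
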(event `self.OnSphereBeginOverlap`
  (add `self.OnActorHit` (delegate `OnActorHit_Event`)))

(event `OnActorHit_Event` :!signature `self.OnActorHit`
  (params (SelfActor :type "Actor Object Reference") (OtherActor :type "Actor Object Reference") (NormalImpulse :type "Vector Structure") (Hit :type "HitResult Structure (by ref)"))
  (cast `/Game/Blueprints/BlasterBeam/BP_BlasterBeam` OtherActor)
  (if (not (`self.DestroyActor`))
    (set `self.DestroyActor` true)
    (bind _returnvalue (`|SpawnActorFromClass` (`self.ParticleSystem_Pickup_ToSpawn_AtOverlap`) (`self.GetTransform`) "Undefined" "MultiplyWithRoot" null null))
    (`|ExecutionSequence`
      (:`then_0`
        (bind _output_get (set `self.ExplosionParticleEffects` _returnvalue))
        (`self.SetActorRelativeScale3D` _output_get (`self.New Relative Scale`)))
      (:`then_1`
        (`GameplayStatics.SpawnSoundAtLocation` "/Game/SmallSoundKit/SSKCue/MagicCue/Mgc_Electric_Impact_01_Cue.Mgc_Electric_Impact_01_Cue" (`self.K2_GetActorLocation`) (struct) 0.5 0.4 0.0 null null))
      (:`then_2`
        (`KismetSystemLibrary.Delay` (`self.DelayToDestroy`))
        (`self.K2_DestroyActor`)))))

(fn `UserConstructionScript`
  (`parent.UserConstructionScript`))