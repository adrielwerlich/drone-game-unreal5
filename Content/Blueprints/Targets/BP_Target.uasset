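; BP_Target is a shootable target actor that explodes when hit by the first-person projectile.
; A hit on its collision sphere matches the other actor's class display name against BP_FirstPersonProjectile_C, then spawns an explosion particle and sound at the target's location and destroys it.
; Hits on the sphere and mesh also write debug log messages.
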(event `self.Collision_Sphere.OnComponentHit`
  (params (HitComponent :type "PrimitiveComponent Object Reference") (OtherActor :type "Actor Object Reference") (OtherComp :type "PrimitiveComponent Object Reference") (NormalImpulse :type "Vector Structure") (Hit :type "HitResult Structure (by ref)"))
  (bind _returnvalue (`self.K2_GetActorLocation`))
  (`|ExecutionSequence`
    (:`then_0`
      (`KismetSystemLibrary.LogString` "Hello"))
    (:`then_1`
      (if (`KismetStringLibrary.EqualEqual_StrStr` (`KismetSystemLibrary.GetClassDisplayName` (`GameplayStatics.GetObjectClass` OtherActor)) "BP_FirstPersonProjectile_C")
        (`GameplayStatics.SpawnEmitterAtLocation` "/Game/FXVarietyPack/Particles/P_ky_explosion.P_ky_explosion" _returnvalue)
        (`GameplayStatics.SpawnSoundAtLocation` "/Game/StarterContent/Audio/Explosion01.Explosion01" _returnvalue (struct) 1.0 1.0 0.0 null null)
        (`self.K2_DestroyActor`)))))

(event `self.Mesh.OnComponentHit`
  (params (HitComponent :type "PrimitiveComponent Object Reference") (OtherActor :type "Actor Object Reference") (OtherComp :type "PrimitiveComponent Object Reference") (NormalImpulse :type "Vector Structure") (Hit :type "HitResult Structure (by ref)"))
  (`KismetSystemLibrary.LogString` (`KismetSystemLibrary.GetDisplayName` OtherActor)))

(fn `UserConstructionScript`)