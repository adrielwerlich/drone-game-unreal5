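; BP_BlasterBeam is a blaster shot actor that explodes on impact.
; On BeginPlay it binds BeamMesh's hit event, and after a short delay it prints its owner's name and clears ignore-when-moving for that owner.
; A hit prints the other actor, spawns a normal-aligned Niagara explosion and a quiet sound, then destroys the beam.
; Tick is empty, and the forward-offset movement using LaserSpeed is disconnected.
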(event `self.ReceiveBeginPlay`
  (bind _returnvalue (`self.GetOwner`))
  (`|ExecutionSequence`
    (:`then_0`
      (`KismetSystemLibrary.Delay` 0.2)
      (`KismetSystemLibrary.PrintString` (`KismetSystemLibrary.GetDisplayName` _returnvalue))
      (`PrimitiveComponent.IgnoreActorWhenMoving` (`self.BeamMesh`) _returnvalue false))
    (:`then_1`
      (add `PrimitiveComponent.OnComponentHit` (`self.BeamMesh`) (delegate `OnComponentHit_Event`)))))

(event `OnComponentHit_Event`
  (params (HitComponent :type "PrimitiveComponent Object Reference") (OtherActor :type "Actor Object Reference") (OtherComp :type "PrimitiveComponent Object Reference") (NormalImpulse :type "Vector Structure") (Hit :type "HitResult Structure (by ref)"))
  (bind (_bblockinghit _binitialoverlap _time _distance _location _impactpoint _normal) (`GameplayStatics.BreakHitResult` Hit))
  (`KismetSystemLibrary.PrintString` (`KismetSystemLibrary.GetDisplayName` OtherActor))
  (`NiagaraFunctionLibrary.SpawnSystemAtLocation` "/Game/FX/NS_HitExplosion.NS_HitExplosion" _impactpoint (`KismetMathLibrary.MakeRotFromX` _normal))
  (`GameplayStatics.SpawnSoundAtLocation` "/Game/StarterContent/Audio/Explosion02.Explosion02" _location (struct) 0.1 1.0 0.0 null null)
  (`self.K2_DestroyActor`))

(event `self.ReceiveTick`
  (params (DeltaSeconds :type "Float (single-precision)")))

(fn `UserConstructionScript`)