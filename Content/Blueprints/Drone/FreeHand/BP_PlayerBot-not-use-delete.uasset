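; Enemy-style bot actor that turns to face the first DefaultPawn in the level and fires blaster beams; the asset name marks it as unused.
; Tick eases rotation toward that pawn with a randomized interpolation speed.
; After a short startup delay, a looping timer spawns BP_BlasterBeam and Niagara bursts at both rifle sockets.
; Only the right beam gets the bot as owner and ignores its mesh when moving.
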(event `SpawnBlasterBeam`
  (`|ExecutionSequence`
    (:`then_0`
      (bind _output_get (set `self.LeftRifleTransform` (`SceneComponent.GetSocketTransform` (`self.BotMesh`) (`self.LeftRifleSocketName`) "RTS_World"))))
    (:`then_1`
      (bind _output_get_2 (set `self.RightRifleTransform` (`SceneComponent.GetSocketTransform` (`self.BotMesh`) (`self.RightRifleSocketName`) "RTS_World"))))
    (:`then_2`
      (`|SpawnActorFromClass` "/Game/Blueprints/BlasterBeam/BP_BlasterBeam.BP_BlasterBeam_C" _output_get "Undefined" "MultiplyWithRoot" null null)
      (bind _returnvalue (`|SpawnActorFromClass` "/Game/Blueprints/BlasterBeam/BP_BlasterBeam.BP_BlasterBeam_C" _output_get_2 "Undefined" "MultiplyWithRoot" null null))
      (bind _output_get_3 (set `self.Laser` _returnvalue))
      (`self.SetOwner` _output_get_3 self)
      (`PrimitiveComponent.IgnoreComponentWhenMoving` (`/Game/Blueprints/BlasterBeam/BP_BlasterBeam.BeamMesh` (`self.Laser`)) (`self.BotMesh`) true)
      (`NiagaraFunctionLibrary.SpawnSystemAttached` "/Game/FX/NS_BeamBurst.NS_BeamBurst" (`self.BotMesh`) (`self.RightRifleSocketName`) (0.0 0.0 0.0) (struct) "KeepRelativeOffset")
      (`NiagaraFunctionLibrary.SpawnSystemAttached` "/Game/FX/NS_BeamBurst.NS_BeamBurst" (`self.BotMesh`) (`self.LeftRifleSocketName`) (0.0 0.0 0.0) (struct) "KeepRelativeOffset"))))

(event `self.ReceiveBeginPlay`
  (`self.StoreTargetPawn`)
  (`KismetSystemLibrary.Delay` 0.5)
  (`KismetSystemLibrary.K2_SetTimerDelegate` (delegate `SpawnBlasterBeam`) 0.3 true))

(event `self.ReceiveTick`
  (params (DeltaSeconds :type "Float (single-precision)"))
  (`self.InterpolateRotation` DeltaSeconds (`self.Interpolation Speed`))
  (set `self.Interpolation Speed` (`KismetMathLibrary.RandomFloatInRange` 3.0 9.0)))

(fn `FindTargetRotation`
  (returns (ReturnValue :type "Rotator Structure"))
  (return (`KismetMathLibrary.FindLookAtRotation` (`self.K2_GetActorLocation`) (`self.K2_GetActorLocation` (`self.TargetPawn`)))))

(fn `InterpolateRotation`
  (params (DeltaTime :type "Float (single-precision)") (InterpolationSpeed :type "Float (double-precision)"))
  (`self.TargetPawn`
    (:`then`
      (`self.K2_SetActorRotation` (`KismetMathLibrary.RInterpTo` (`self.K2_GetActorRotation`) (`self.FindTargetRotation`) DeltaTime InterpolationSpeed)))
    (:`else`)))

(fn `StoreTargetPawn`
  (bind _outactors (`GameplayStatics.GetAllActorsOfClass` "/Script/Engine.DefaultPawn"))
  (if (`KismetArrayLibrary.Array_IsValidIndex` _outactors)
    (set `self.TargetPawn` (`|GetArrayItem` _outactors))
    (return)))

(fn `UserConstructionScript`)